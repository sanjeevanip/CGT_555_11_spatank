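; BP_ChaosFieldController is a destruction sequencer that fires a list of Chaos field actors in timed order.
; Toggle and CallTriggerActor share one path that waits briefly, then calls CETrigger on up to six valid Fields entries, spaced by a configurable Delay.
; The sequence is hand-unrolled rather than looped, and after DisableDelay it sets FieldActive to true on the referenced Disable field.
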(event EventToggle
  (params (On/off :type Boolean))
  (bind _disable (Variables|Default|Getdisable))
  (bind _fields (Variables|Default|GetFields))
  (bind _fields_2 (Variables|Default|GetFields))
  (bind _fields_3 (Variables|Default|GetFields))
  (bind _fields_4 (Variables|Default|GetFields))
  (bind _fields_5 (Variables|Default|GetFields))
  (bind _fields_6 (Variables|Default|GetFields))
  (bind _output (Utilities|Array|Get(acopy) _fields_2 3))
  (bind _output_2 (Utilities|Array|Get(acopy) _fields_3 4))
  (bind _output_3 (Utilities|Array|Get(acopy) _fields_6 5))
  (bind _output_4 (Utilities|Array|Get(acopy) _fields_4))
  (bind _output_5 (Utilities|Array|Get(acopy) _fields_5 1))
  (bind _output_6 (Utilities|Array|Get(acopy) _fields 2))
  (Variables|Default|SetnumFields (Utilities|Array|Length (Variables|Default|GetFields)))
  (if (> (Variables|Default|GetnumFields) 0)
    (Utilities|FlowControl|Delay 1.0)
    (Utilities|IsValid _output_4
      (:Is%20Valid
        (Default|CETrigger _output_4)
        (Utilities|FlowControl|Delay (Variables|Default|GetDelay)))
      (:Is%20Not%20Valid
        _))
    (if (> (Variables|Default|GetnumFields) 1)
      (Utilities|IsValid _output_5
        (:Is%20Valid
          (Default|CETrigger _output_5)
          (Utilities|FlowControl|Delay (Variables|Default|GetDelay)))
        (:Is%20Not%20Valid
          _)))
    (if (> (Variables|Default|GetnumFields) 2)
      (Utilities|IsValid _output_6
        (:Is%20Valid
          (Default|CETrigger _output_6)
          (Utilities|FlowControl|Delay (Variables|Default|GetDelay)))
        (:Is%20Not%20Valid
          _)))
    (if (> (Variables|Default|GetnumFields) 3)
      (Utilities|IsValid _output
        (:Is%20Valid
          (Default|CETrigger _output)
          (Utilities|FlowControl|Delay (Variables|Default|GetDelay)))
        (:Is%20Not%20Valid
          _)))
    (if (> (Variables|Default|GetnumFields) 4)
      (Utilities|IsValid _output_2
        (:Is%20Valid
          (Default|CETrigger _output_2)
          (Utilities|FlowControl|Delay (Variables|Default|GetDelay)))
        (:Is%20Not%20Valid
          _)))
    (if (> (Variables|Default|GetnumFields) 5)
      (Utilities|IsValid _output_3
        (:Is%20Valid
          (Default|CETrigger _output_3))
        (:Is%20Not%20Valid
          _)))
    (Utilities|FlowControl|Delay (Variables|Default|GetDisableDelay))
    (Utilities|IsValid _disable
      (:Is%20Valid
        (Variables|/Engine/EditorResources/FieldNodes/FS_SleepDisable_Generic.FS_SleepDisable_Generic_C|SetField%20Active _disable true)))))

(event EventCallTriggerActor
  (bind _disable (Variables|Default|Getdisable))
  (bind _fields (Variables|Default|GetFields))
  (bind _fields_2 (Variables|Default|GetFields))
  (bind _fields_3 (Variables|Default|GetFields))
  (bind _fields_4 (Variables|Default|GetFields))
  (bind _fields_5 (Variables|Default|GetFields))
  (bind _fields_6 (Variables|Default|GetFields))
  (bind _output (Utilities|Array|Get(acopy) _fields_2 3))
  (bind _output_2 (Utilities|Array|Get(acopy) _fields_3 4))
  (bind _output_3 (Utilities|Array|Get(acopy) _fields_6 5))
  (bind _output_4 (Utilities|Array|Get(acopy) _fields_4))
  (bind _output_5 (Utilities|Array|Get(acopy) _fields_5 1))
  (bind _output_6 (Utilities|Array|Get(acopy) _fields 2))
  (Variables|Default|SetnumFields (Utilities|Array|Length (Variables|Default|GetFields)))
  (if (> (Variables|Default|GetnumFields) 0)
    (Utilities|FlowControl|Delay 1.0)
    (Utilities|IsValid _output_4
      (:Is%20Valid
        (Default|CETrigger _output_4)
        (Utilities|FlowControl|Delay (Variables|Default|GetDelay)))
      (:Is%20Not%20Valid
        _))
    (if (> (Variables|Default|GetnumFields) 1)
      (Utilities|IsValid _output_5
        (:Is%20Valid
          (Default|CETrigger _output_5)
          (Utilities|FlowControl|Delay (Variables|Default|GetDelay)))
        (:Is%20Not%20Valid
          _)))
    (if (> (Variables|Default|GetnumFields) 2)
      (Utilities|IsValid _output_6
        (:Is%20Valid
          (Default|CETrigger _output_6)
          (Utilities|FlowControl|Delay (Variables|Default|GetDelay)))
        (:Is%20Not%20Valid
          _)))
    (if (> (Variables|Default|GetnumFields) 3)
      (Utilities|IsValid _output
        (:Is%20Valid
          (Default|CETrigger _output)
          (Utilities|FlowControl|Delay (Variables|Default|GetDelay)))
        (:Is%20Not%20Valid
          _)))
    (if (> (Variables|Default|GetnumFields) 4)
      (Utilities|IsValid _output_2
        (:Is%20Valid
          (Default|CETrigger _output_2)
          (Utilities|FlowControl|Delay (Variables|Default|GetDelay)))
        (:Is%20Not%20Valid
          _)))
    (if (> (Variables|Default|GetnumFields) 5)
      (Utilities|IsValid _output_3
        (:Is%20Valid
          (Default|CETrigger _output_3))
        (:Is%20Not%20Valid
          _)))
    (Utilities|FlowControl|Delay (Variables|Default|GetDisableDelay))
    (Utilities|IsValid _disable
      (:Is%20Valid
        (Variables|/Engine/EditorResources/FieldNodes/FS_SleepDisable_Generic.FS_SleepDisable_Generic_C|SetField%20Active _disable true)))))

(fn ConstructionScript)