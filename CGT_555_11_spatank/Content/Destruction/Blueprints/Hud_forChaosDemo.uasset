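; HUD for the Chaos destruction demo that draws a crosshair in the center of the screen.
; Each DrawHUD call casts the player character to PlayerCharacter_Physics and checks its CanFire flag.
; While firing is possible, it draws the M_Crosshair material at a fixed pixel size, offset by half that size from the viewport center.
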(event EventDrawHUD
  (params (SizeX :type Integer) (SizeY :type Integer))
  (bind _returnvalue (Math|Float|MakeLiteralFloat 4e+01))
  (bind _returnvalue_2 (/ _returnvalue 2.0))
  ;[1 1 1] Draw Crosshair in the center of the screen when aiming is possible
  (bind _asplayer_character_physics (Utilities|Casting|CastToPlayerCharacter_Physics (Game|GetPlayerCharacter 0)))
  (if (Variables|/Game/Destruction/Blueprints/PlayerCharacter_Physics.PlayerCharacter_Physics_C|GetbCanFire _asplayer_character_physics)
    (Canvas|DrawMaterial "/Game/Destruction/Materials/M_Crosshair.M_Crosshair" (- (/ (Math|Conversions|ToFloat(Integer) SizeX) 2.0) _returnvalue_2) (- (/ (Math|Conversions|ToFloat(Integer) SizeY) 2.0) _returnvalue_2) _returnvalue _returnvalue 0.0 0.0 1.0 1.0)))

(fn ConstructionScript)