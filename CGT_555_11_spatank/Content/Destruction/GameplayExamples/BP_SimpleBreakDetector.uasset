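; Example actor that monitors a referenced Geometry Collection for Chaos break events and visualizes them.
; It binds to OnChaosBreakEvent, turning its status text and preview sphere green on detection and optionally drawing velocity-tinted debug spheres at each break.
; It also accumulates broken mass for an optional text readout.
; It can warn on screen when NotifyBreaks is off, and a trigger interface call enables that flag once.
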(event Custom|OnBreakEvent
  (params (BreakEvent :type Chaos%20Break%20Event%20Structure%20%28by%20ref%29))
  (bind (_component _location _velocity _angularvelocity _mass) (Utilities|Struct|BreakChaosBreakEvent BreakEvent))
  (bind _color (Math|Color|MakeColor 0 255 0))
  (bind _statusmessage (Variables|Default|GetStatusMessage))
  (bind _returnvalue (Math|Vector|VectorLength _velocity))
  (bind _returnvalue_2 (Math|Float|MapRangeClamped _returnvalue 0.0 5e+02 0.0 1.0))
  (Rendering|Components|TextRender|SetText _statusmessage (Utilities|Text|MakeLiteralText "Detected!"))
  (Rendering|Components|TextRender|SetTextRenderColor _statusmessage _color)
  (Rendering|Material|SetVectorParameterValue (Variables|Default|GetSphere%20Colour) "Colour" (Math|Conversions|ToLinearColor(Color) _color) :!class /Script/Engine.MaterialInstanceDynamic)
  ;[1 1 1 1 14] The ChaosBreakEvent struct reports all relevant information about the breaks in the GeometryCollection. Here we map the velocity (== size) of each break into a 0-1 range and draw debug spheres of matching sizes to visualize each break.
  (Utilities|FlowControl|Sequence
    (:then_0
      (if (Variables|Default|GetVisualizeBreaks)
        (Rendering|Debug|DrawDebugSphere _location 25.0 12 (Utilities|Struct|MakeLinearColor 1.0 _returnvalue_2 _returnvalue_2 1.0) 1e+03)))
    (:then_1
      ;[1 1 1 1 14] Since each break creates its own event, we can accumulate all of them into a counter for the final mass.
      (Variables|Mass|SetMassGenerated (+ _mass (Variables|Mass|GetMassGenerated)))
      (if (Variables|Default|GetVisualizeMass)
        (CallFunction|UpdateMassStatus)
        (Rendering|SetVisibility (Variables|Default|GetMassStatus) true false)))))

(event EventBeginPlay
  (bind _geometrycollectiontomonitor (Variables|Default|GetGeometryCollectionToMonitor))
  (bind _geometrycollectioncomponent (Variables|/Script/GeometryCollectionEngine.GeometryCollectionActor|GetGeometryCollectionComponent _geometrycollectiontomonitor))
  (CallFunction|InitStatusMessage)
  ;[1 1 1 1 14] Subscribe to a GeometryCollectionComponent's built-in OnChaosBreakEvent event to act on each structural breal that gets recorded.
  (EventDispatchers|BindEventtoOnChaosBreakEvent _geometrycollectioncomponent (delegate Custom|OnBreakEvent))
  ;[1 1 1 1 14] Users might forget to enable the NotifyCollisions flag on the GeometryCollection you want to monitor. We usually warn them via a dev-only on-screen message.
  (if (not (Variables|/Script/GeometryCollectionEngine.GeometryCollectionComponent|GetbNotifyBreaks _geometrycollectioncomponent))
    (if (Variables|Default|GetEnable%20On-Screen%20Warnings)
      (Development|PrintString (Utilities|String|Append "Warning! Trying to monitor '" (Utilities|GetDisplayName (Variables|/Script/GeometryCollectionEngine.GeometryCollectionActor|GetGeometryCollectionComponent (Variables|Default|GetGeometryCollectionToMonitor))) "' for breaks, but the component is not sending them!") true true "(R=0.000000,G=0.660000,B=1.000000,A=1.000000)" 6.0))))

(event EventCallTriggerActor
  ;[1 1 1 1 14] Support triggers turning on the NotifyBreaks flag.
  (Utilities|FlowControl|DoOnce false
    (:Completed
      (Class|GeometryCollectionComponent|SetNotifyBreaks (Variables|/Script/GeometryCollectionEngine.GeometryCollectionActor|GetGeometryCollectionComponent (Variables|Default|GetGeometryCollectionToMonitor)) true)
      (CallFunction|InitStatusMessage))))

(fn ConstructionScript
  (bind _returnvalue (Rendering|Material|CreateDynamicMaterialInstance (Variables|Default|GetSphere) 0 "/Game/Destruction/Materials/M_Preview_BreakEvents.M_Preview_BreakEvents" "None" :!class /Script/Engine.PrimitiveComponent))
  (bind _output_get (Variables|Default|SetSphere%20Colour _returnvalue))
  (Rendering|Material|SetVectorParameterValue _output_get "Colour" "(R=1.000000,G=1.000000,B=1.000000,A=1.000000)" :!class /Script/Engine.MaterialInstanceDynamic))

(fn InitStatusMessage
  (bind _color (Math|Color|MakeColor 0 0 255))
  (bind _color_2 (Math|Color|MakeColor 0 100 255))
  (bind _statusmessage (Variables|Default|GetStatusMessage))
  (bind _geometrycollectiontomonitor (Variables|Default|GetGeometryCollectionToMonitor))
  (bind _geometrycollectioncomponent (Variables|/Script/GeometryCollectionEngine.GeometryCollectionActor|GetGeometryCollectionComponent _geometrycollectiontomonitor))
  (bind _bnotifybreaks (Variables|/Script/GeometryCollectionEngine.GeometryCollectionComponent|GetbNotifyBreaks _geometrycollectioncomponent))
  (bind _returnvalue (select _bnotifybreaks _color_2 _color))
  (Rendering|Components|TextRender|SetText _statusmessage (select _bnotifybreaks (Variables|Default|GetEventsGetGeneratedText) (Variables|Default|GetNoEventsGeneratedText)))
  (Rendering|Components|TextRender|SetTextRenderColor _statusmessage _returnvalue)
  (Rendering|Material|SetVectorParameterValue (Variables|Default|GetSphere%20Colour) "Colour" (Math|Conversions|ToLinearColor(Color) _returnvalue) :!class /Script/Engine.MaterialInstanceDynamic))

(fn UpdateMassStatus
  (Rendering|Components|TextRender|SetText (Variables|Default|GetMassStatus) (Utilities|Text|ToText(String) (Utilities|String|Append (Variables|Default|GetMassGeneratedText) (Utilities|String|ToString(Integer) (Math|Float|Truncate (Variables|Mass|GetMassGenerated))))))
  (Rendering|SetVisibility (Variables|Default|GetMassStatus) true false)
  (Rendering|Components|TextRender|SetTextRenderColor (Variables|Default|GetMassStatus) (Math|Color|MakeColor 0 255 0)))